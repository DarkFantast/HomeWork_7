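; BP_DestroyCube is an actor with hit points that wears down and is destroyed as BP_Ball actors overlap it.
; On BeginPlay it divides BaseHP by HP and stores the result back in BaseHP as the damage per hit.
; Each ball overlap destroys the cube if HP is already at or below DestroyHP, and otherwise subtracts that damage from HP.
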(event `self.ReceiveBeginPlay`
  (set `self.BaseHP` (* (/ (`self.BaseHP`) (`self.%HP`)) 1.0)))

(event `self.ReceiveActorBeginOverlap`
  (params (OtherActor :type "Actor Object Reference"))
  (cast `/Game/BP_Ball` OtherActor)
  (if (<= (`self.HP`) (`self.DestroyHP`))
    (`self.K2_DestroyActor`)
    (else
      (set `self.HP` (- (`self.HP`) (`self.BaseHP`))))))

(fn `UserConstructionScript`)